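; Connect button actor that plays an animated "Connect" word and starts joining an online multiplayer session.
; StartMenuAnimation plays the word's animation once.
; OnConnectClicked runs a non-LAN FindSessions with debug prints, then attempts JoinSession on the first result, even when the search fails.
; A looping Host idle animation node is left unconnected and never runs.
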(event Custom|StartMenuAnimation
  (Components|Animation|PlayAnimation (Variables|Default|GetConnect_word_anim_Play) "/Game/Geometry/Meshes/Animated/Connect_BTN/Connect_word_anim_Play_Anim.Connect_word_anim_Play_Anim" false))

(event Custom|OnConnectClicked
  (bind _results (|FindSessions (Game|GetPlayerController 0) 5 false)
    (:OnSuccess
      (Development|PrintString (Utilities|String|Append "FIND SESSION SUCCESS" (Utilities|String|ToString(Integer) (Utilities|Array|Length _results)))))
    (:OnFailure
      (Development|PrintString "FIND SESSION FAILURE")))
  (|JoinSession (Game|GetPlayerController 0) (Utilities|Array|Get(acopy) _results)))

(event EventBeginPlay)

(event Collision|EventActorBeginOverlap
  (params (OtherActor :type Actor%20Object%20Reference)))

(event EventTick
  (params (DeltaSeconds :type Float%20%28single-precision%29)))

(fn ConstructionScript)
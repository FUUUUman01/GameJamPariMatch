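; BallSpawner is a networked, player-owned actor that spawns balls and shows its owner's color on its Truba component.
; Spawn creates a BallClass actor at the Sphere's world transform, passing OwnerPlayerState as owner and as a spawn parameter.
; The owner's PlayerIndex selects a data table row whose BallColor sets Truba's material Color.
; Coloring runs on BeginPlay if the owner is valid, or when OwnerPlayerState's RepNotify fires.
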(event Custom|Spawn
  (bind _ownerplayerstate (Variables|Default|GetOwnerPlayerState))
  (Game|SpawnActorfromClass (Variables|Default|GetBallClass) (Transformation|GetWorldTransform (Variables|Default|GetSphere)) "Undefined" _ownerplayerstate _ownerplayerstate 0))

(event Custom|OnPlayerStateSet
  (bind _returnvalue (Utilities|GetDataTableRow "/Game/Blueprints/PlayerIDColorDataTable.PlayerIDColorDataTable" (Utilities|String|StringToName (Utilities|String|ToString(Integer) (Variables|/Game/Blueprints/BP_PlayerState.BP_PlayerState_C|GetPlayerIndex (Variables|Default|GetOwnerPlayerState)))))
    (:then
      (Rendering|Material|SetVectorParameterValueonMaterials (Variables|Default|GetTruba) "Color" (Math|Vector|MakeVector (.r (.ballcolor _returnvalue)) (.g (.ballcolor _returnvalue)) (.b (.ballcolor _returnvalue)))))))

(event EventBeginPlay
  (Variables|Default|GetOwnerPlayerState
    (:then
      (bind _returnvalue (Utilities|GetDataTableRow "/Game/Blueprints/PlayerIDColorDataTable.PlayerIDColorDataTable" (Utilities|String|StringToName (Utilities|String|ToString(Integer) (Variables|/Game/Blueprints/BP_PlayerState.BP_PlayerState_C|GetPlayerIndex (Variables|Default|GetOwnerPlayerState)))))
        (:then
          (Rendering|Material|SetVectorParameterValueonMaterials (Variables|Default|GetTruba) "Color" (Math|Vector|MakeVector (.r (.ballcolor _returnvalue)) (.g (.ballcolor _returnvalue)) (.b (.ballcolor _returnvalue)))))))
    (:else)))

(event Collision|EventActorBeginOverlap
  (params (OtherActor :type Actor%20Object%20Reference)))

(fn ConstructionScript)

(fn HasValidPlayerStateOwner
  (return (Utilities|IsValid (Variables|Default|GetOwnerPlayerState))))

(fn OnRepOwnerPlayerState
  (CallFunction|OnPlayerStateSet))
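; Player state for a multiplayer betting game, holding each player's money, current bets, ready flag and player index.
; RepNotify handlers for money, readiness and index broadcast dispatchers to listeners.
; PlaceBet totals the submitted bets, then deducts the sum and stores them if affordable, otherwise only printing an error.
; ResetBets clears the stored bets without refunding and multicasts a reset notification.
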(event Custom|PlaceBet
  (params (Bets :type Array%20of%20F%20Bet%20Struct%20Structures))
  (CallFunction|ImplPlaceBet Bets))

(event Custom|MulticastResetBets
  (Default|CallOnResetBets))

(fn ConstructionScript)

(fn OnRepIsReady
  (Default|CallOnReadyChanged (Variables|Default|GetIsReady)))

(fn OnRepPlayerIndex
  (Default|CallOnPlayerIndexInit (Variables|Default|GetPlayerIndex)))

(fn SetMoney
  (params (NewMoney :type Integer))
  (Variables|Default|SetMoney NewMoney))

(fn OnRepMoney
  (Default|CallOnMoneyChanged (Variables|Default|GetMoney)))

(fn ResetBets
  (Utilities|Array|Clear (Variables|Default|GetBets))
  (CallFunction|MulticastResetBets))

(fn ImplPlaceBet
  (params (InBets :type Array%20of%20F%20Bet%20Struct%20Structures))
  (LocalVariables|SetTotalBet 0)
  (for _array_element InBets
    (LocalVariables|SetTotalBet (+ (.Bet (Utilities|Struct|BreakFBetStruct _array_element)) (LocalVariables|GetTotalBet))))
  (bind _output_get (LocalVariables|SetNewMoney (- (Variables|Default|GetMoney) (LocalVariables|GetTotalBet))))
  (if (>= _output_get 0)
    (CallFunction|SetMoney (LocalVariables|GetNewMoney))
    (Variables|Default|SetBets InBets)
    (else
      (Development|PrintString "ERROR ImplPlaceBet"))))
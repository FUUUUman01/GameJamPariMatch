(event Custom|ExitBuildingMod
  (Variables|Default|SetbShowMouseCursor false)
  (Input|SetIgnoreLookInput false)
  (Variables|Default|SetbIsBuilding false)
  (Class|PlayerController|SetVirtualJoystickVisibility false)
  (Default|CallOnChangedBuildingModClient false 0.0))

(event Custom|EnterBuildingModServer
  (params (BuildTime :type Float%20%28single-precision%29))
  (CallFunction|EnterBuildingModClient BuildTime)
  (Variables|Default|SetbIsBuilding true))

(event Custom|EnterBuildingModClient
  (params (BuildTime :type Float%20%28single-precision%29))
  (Variables|Default|SetbShowMouseCursor true)
  (Input|SetIgnoreLookInput true)
  (Variables|Default|SetbIsBuilding true)
  (Class|PlayerController|SetVirtualJoystickVisibility false)
  (Default|CallOnChangedBuildingModClient true BuildTime))

(event Custom|TraceForPlacable
  (bind (_worldlocation _worlddirection) (Game|Player|ConvertMouseLocationToWorldSpace))
  (bind _outhit (Collision|LineTraceByChannel _worldlocation (+ _worldlocation (* _worlddirection 1e+05)) "TraceTypeQuery3" false 0 "None"))
  (if (.bblockinghit _outhit)
    (bind _asplacable_object_base (Utilities|Casting|CastToPlacableObjectBase (.hitactor _outhit))
      (:then
        (CallFunction|TrySelectObject _asplacable_object_base))
      (:CastFailed
        (if (CallFunction|IsMineBuildingGrid (.hitactor _outhit))
          (CallFunction|SpawnPlacableRPC (Variables|Default|GetCurrentPlacableItem) (Math|Transform|MakeTransform (.location _outhit))))))))

(event Custom|SpawnPlacableRPC
  (params (Class :type Placable%20Object%20Base%20Class%20Reference) (SpawnTransform :type Transform))
  (bind _asbp_player_state (Utilities|Casting|CastToBP_PlayerState (Variables|GetPlayerState)))
  (bind _returnvalue (Game|SpawnActorfromClass Class SpawnTransform "AlwaysSpawn" self _asbp_player_state 0))
  (Default|PaintObject _returnvalue)
  (Utilities|Array|Add (Variables|Default|GetMyPlacableObjects) _returnvalue))

(event Custom|RequestStopBuildingClient
  (if (Variables|Default|GetbIsBuilding)
    (CallFunction|ExitBuildingModServer)))

(event Custom|SetIsReadyServer
  (params (NewReady :type Boolean))
  (bind _asbp_player_state (Utilities|Casting|CastToBP_PlayerState (Variables|GetPlayerState)))
  (Variables|/Game/Blueprints/BP_PlayerState.BP_PlayerState_C|SetIsReady _asbp_player_state NewReady))

(event Custom|ExitBuildingModServer
  (Variables|Default|SetbIsBuilding false)
  (Default|CallOnClientStoppedBuildingServer self)
  (CallFunction|ExitBuildingMod))

(event EventBeginPlay
  (bind _self self)
  (if (Pawn|IsLocalPlayerController)
    (bind _returnvalue (UserInterface|CreateWidget "/Game/Blueprints/Widgets/PlayerHUD.PlayerHUD_C" _self _self))
    (UserInterface|Viewport|AddtoViewport _returnvalue 0)
    (Variables|Default|SetHUDRef _returnvalue)))

(event EventTick
  (params (DeltaSeconds :type Float%20%28single-precision%29))
  (bind (_worldlocation _worlddirection) (Game|Player|ConvertMouseLocationToWorldSpace))
  (if (Variables|Default|GetbIsBuilding)
    (Utilities|FlowControl|Sequence
      (:then_0
        (bind _currentselectedobject (Variables|Default|GetCurrentSelectedObject)
          (:then
            (Development|PrintString (Utilities|GetDisplayName _currentselectedobject))
            (bind (_outhit _returnvalue) (Collision|LineTraceByChannel _worldlocation (+ _worldlocation (* _worlddirection 1e+05)) "TraceTypeQuery4" false 0 "None"))
            (if (and _returnvalue (CallFunction|IsMineBuildingGrid (.HitActor (Collision|BreakHitResult _outhit))))
              (if (Variables|Default|GetRotateObject)
                (Transformation|SetActorRotation (Variables|Default|GetCurrentSelectedObject) (Math|Rotator|MakeRotator (.roll (Math|Rotator|FindLookatRotation (Transformation|GetActorLocation (Variables|Default|GetCurrentSelectedObject)) (.Location (Collision|BreakHitResult _outhit)))) (.pitch (Math|Rotator|FindLookatRotation (Transformation|GetActorLocation (Variables|Default|GetCurrentSelectedObject)) (.Location (Collision|BreakHitResult _outhit)))) (.yaw (Math|Rotator|FindLookatRotation (Transformation|GetActorLocation (Variables|Default|GetCurrentSelectedObject)) (.Location (Collision|BreakHitResult _outhit))))))
                (else
                  (Transformation|SetActorLocation (Variables|Default|GetCurrentSelectedObject) (.Location (Collision|BreakHitResult _outhit)) false false)))))
          (:else)))
      (:then_1
        (if (Pawn|IsLocalPlayerController)
          (for _array_element (Variables|Default|GetMyPlacableObjects)
            (Default|CheckIsValidPosition _array_element)))))))

(event Input|KeyboardEvents|E
  (params (Key :type Key%20Structure :default "None"))
  (:Pressed
    (CallFunction|EnterBuildingModClient 0.0))
  (:Released
    (CallFunction|ExitBuildingMod)))

(event Input|MouseEvents|LeftMouseButton
  (params (Key :type Key%20Structure :default "None"))
  (:Pressed
    (if (Variables|Default|GetbIsBuilding)
      (CallFunction|TraceforPlacable)))
  (:Released
    (CallFunction|DeselectPlacableObject)))

(event Input|TouchEvents|InputTouch
  (params (Location :type Vector) (FingerIndex :type ETouchIndex%20Enum))
  (:Pressed
    (if (Variables|Default|GetbIsBuilding)
      (CallFunction|TraceforPlacable)))
  (:Released
    (CallFunction|DeselectPlacableObject)))

(fn ConstructionScript)

(fn ToggleBuildingMode
  (if (Variables|Default|GetbIsBuilding)
    (CallFunction|ExitBuildingMod)
    (else
      (CallFunction|EnterBuildingModClient 0.0))))

(fn SelectPlacableObject
  (params (Object :type Placable%20Object%20Base%20Object%20Reference))
  (CallFunction|DeselectPlacableObject)
  (bind _output_get (Variables|Default|SetCurrentSelectedObject Object))
  (Default|CallOnObjectSelected _output_get))

(fn DeselectPlacableObject
  (Variables|Default|SetCurrentSelectedObject 0)
  (Default|CallOnObjectSelected))

(fn TrySelectObject
  (params (TrySelectObject :type Placable%20Object%20Base%20Object%20Reference))
  (Variables|/Game/Blueprints/PlacableObjects/PlacableObjectBase.PlacableObjectBase_C|GetOwnerPlayerState TrySelectObject
    (:then
      (if (and (!= TrySelectObject (Variables|Default|GetCurrentSelectedObject)) (== (Variables|/Game/Blueprints/BP_PlayerState.BP_PlayerState_C|GetPlayerIndex (.AsBP%20Player%20State (Utilities|Casting|CastToBP_PlayerState (Variables|GetPlayerState)))) (Variables|/Game/Blueprints/BP_PlayerState.BP_PlayerState_C|GetPlayerIndex (Variables|/Game/Blueprints/PlacableObjects/PlacableObjectBase.PlacableObjectBase_C|GetOwnerPlayerState TrySelectObject))))
        (CallFunction|SelectPlacableObject TrySelectObject)
        (else
          (CallFunction|DeselectPlacableObject))))
    (:else)))

(fn IsMineBuildingGrid
  (params (Grid :type Actor%20Object%20Reference))
  (bind _asbuild_grid (Utilities|Casting|CastToBuildGrid Grid)
    (:then
      (return (== (Variables|/Game/Blueprints/BuildGrid.BuildGrid_C|GetOwnerPlayerState _asbuild_grid) (Variables|GetPlayerState))))
    (:CastFailed
      (return false))))
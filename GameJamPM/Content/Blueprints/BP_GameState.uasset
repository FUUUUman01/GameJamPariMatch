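; Game state for a betting game, handling game phase, winner notifications and bet payouts.
; Client events relay phase changes and player wins through event dispatchers, and a separate handler stores the current phase.
; GiveOutPrize pools all players' bets and splits the bank among the winner's backers in proportion to their stakes, truncated to whole amounts.
; ResetBetsForAllPlayers clears bets on every player state.
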(event Custom|OnGamePhaseChangedClient
  (params (NewPhase :type EGamePhase%20Enum :default "NewEnumerator2") (OldPhase :type EGamePhase%20Enum :default "NewEnumerator2"))
  (Default|CallOnGamePhaseChanged NewPhase OldPhase))

(event Custom|OnPlayerWinClient
  (params (Player :type BP%20Player%20State%20Object%20Reference))
  (Default|CallOnPlayerWin Player))

(event Custom|OnGamePhaseChanged_Event
  (params (NewPhase :type EGamePhase%20Enum :default "NewEnumerator2") (OldPhase :type EGamePhase%20Enum :default "NewEnumerator2"))
  (Variables|Default|SetCurrentGamePhase NewPhase))

(event EventBeginPlay)

(event EventTick
  (params (DeltaSeconds :type Float%20%28single-precision%29)))

(fn ConstructionScript)

(fn GiveOutPrize
  (params (WinnerId :type Integer))
  (bind _betsonwinner (LocalVariables|GetBetsOnWinner))
  (for _array_element (Variables|Default|GetPlayerArray)
    (bind _asbp_player_state (Utilities|Casting|CastToBP_PlayerState _array_element))
    (for _array_element_2 (Variables|/Game/Blueprints/BP_PlayerState.BP_PlayerState_C|GetBets _asbp_player_state)
      (LocalVariables|SetTotalBank (+ (.Bet (Utilities|Struct|BreakFBetStruct _array_element_2)) (LocalVariables|GetTotalBank)))
      (if (== (.PlayerId (Utilities|Struct|BreakFBetStruct _array_element_2)) WinnerId)
        (Utilities|Map|Add (LocalVariables|GetBetsOnWinner) _asbp_player_state (.Bet (Utilities|Struct|BreakFBetStruct _array_element_2)))
        (LocalVariables|SetTotalBetOnWinner (+ (.Bet (Utilities|Struct|BreakFBetStruct _array_element_2)) (LocalVariables|GetTotalBetOnWinner))))))
  (bind _keys (Utilities|Map|Keys _betsonwinner))
  (bind _values (Utilities|Map|Values _betsonwinner))
  (for (_array_element_3 _array_index) _keys
    (Default|SetMoney _array_element_3 (+ (Variables|/Game/Blueprints/BP_PlayerState.BP_PlayerState_C|GetMoney _array_element_3) (Math|Float|Truncate (* (LocalVariables|GetTotalBank) (/ (Math|Conversions|ToFloat(Integer) (Utilities|Array|Get(acopy) _values _array_index)) (Math|Conversions|ToFloat(Integer) (LocalVariables|GetTotalBetOnWinner)))))))))

(fn ResetBetsforAllPlayers
  (for _array_element (Variables|Default|GetPlayerArray)
    (bind _asbp_player_state (Utilities|Casting|CastToBP_PlayerState _array_element))
    (Default|ResetBets _asbp_player_state)))
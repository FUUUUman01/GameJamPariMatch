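; Placeable rotating bar object that spins two cube components while it is flagged as moving.
; Each Tick calls the parent, then checks IsMoving and adds world-space pitch rotation to both Cube and Cube1, scaled by RotationSpeed and delta time for a frame-rate independent spin.
; The construction script only calls the parent, and the BeginPlay and overlap events are disabled stubs.
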(event EventBeginPlay
  (|CallParentFunction) ; This node is disabled and will not be called.\nDrag off pins to build functionality.
)

(event Collision|EventActorBeginOverlap
  (params (OtherActor :type Actor%20Object%20Reference))
  (|CallParentFunction OtherActor) ; This node is disabled and will not be called.\nDrag off pins to build functionality.
)

(event EventTick
  (params (DeltaSeconds :type Float%20%28single-precision%29))
  (bind _rotationspeed (Variables|Default|GetRotationSpeed))
  (bind _returnvalue (* DeltaSeconds _rotationspeed))
  (|CallParentFunction DeltaSeconds)
  (if (Variables|Default|GetbIsMoving)
    (Transformation|AddWorldRotation (Variables|Default|GetCube) (Math|Rotator|MakeRotator 0.0 _returnvalue 0.0) false false)
    (Transformation|AddWorldRotation (Variables|Default|GetCube1) (Math|Rotator|MakeRotator 0.0 _returnvalue 0.0) false false)))

(fn ConstructionScript
  (|CallParentFunction))
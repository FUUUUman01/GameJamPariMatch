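; Placeable trampoline actor that launches physics components entering its box trigger.
; On box overlap, it replaces the other component's linear velocity with the trampoline's up vector scaled by ImpulseStrength, so the launch follows the actor's rotation.
; A small random offset on each axis of the direction varies every bounce.
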(event OnComponentBeginOverlap(Box)
  (params (OverlappedComponent :type Primitive%20Component%20Object%20Reference) (OtherActor :type Actor%20Object%20Reference) (OtherComp :type Primitive%20Component%20Object%20Reference) (OtherBodyIndex :type Integer) (bFromSweep :type Boolean) (SweepResult :type Hit%20Result%20Structure%20%28by%20ref%29))
  (bind _returnvalue (Transformation|GetActorUpVector))
  (bind (_x _y _z) (Math|Vector|BreakVector _returnvalue))
  (Physics|SetPhysicsLinearVelocity OtherComp (* (Math|Vector|MakeVector (+ _x (Math|Random|RandomFloatinRange -0.1 0.1)) (+ _y (Math|Random|RandomFloatinRange -0.1 0.1)) (+ _z (Math|Random|RandomFloatinRange -0.1 0.1))) (Variables|Default|GetImpulseStrength)) false "None"))

(event EventBeginPlay
  (|CallParentFunction) ; This node is disabled and will not be called.\nDrag off pins to build functionality.
)

(event Collision|EventActorBeginOverlap
  (params (OtherActor :type Actor%20Object%20Reference))
  (|CallParentFunction OtherActor) ; This node is disabled and will not be called.\nDrag off pins to build functionality.
)

(fn ConstructionScript
  (|CallParentFunction))
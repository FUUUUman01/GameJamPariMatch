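; Base actor for placeable objects in a multiplayer game with building phases, handling owner coloring and placement validation.
; On authority, game phase changes clear its placed-this-phase flag.
; A sphere overlap against other placeables sets validity, always true if not placed this phase, and shows the blocking-collision component when invalid.
; RepNotifies refresh that indicator and tint the mesh by player index, with empty mesh and collision getters apparently left for subclasses.
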(event Custom|OnIsValidPositionChanged
  (Rendering|SetVisibility (Variables|Default|GetPlacementBlockingCollision) (not (Variables|Default|GetIsValidPosition)) false))

(event Custom|OnPhaseChanged
  (params (NewPhase :type EGamePhase%20Enum :default "NewEnumerator2") (OldPhase :type EGamePhase%20Enum :default "NewEnumerator2"))
  (bind _output_get (Variables|Default|SetPlacedInThisBuildingPhase false))
  (Default|CallOnPlacedinThisBuildingPhaseChanged _output_get))

(event EventBeginPlay
  (Networking|SwitchHasAuthority
    (:Authority
      (bind _asbp_game_state (Utilities|Casting|CastToBP_GameState (Game|GetGameState)))
      (EventDispatchers|BindEventtoOnGamePhaseChanged _asbp_game_state (delegate Custom|OnPhaseChanged)))))

(event Collision|EventActorBeginOverlap
  (params (OtherActor :type Actor%20Object%20Reference)))

(event EventTick
  (params (DeltaSeconds :type Float%20%28single-precision%29)))

(fn ConstructionScript)

(fn OnRepOwnerPlayerState
  (CallFunction|PaintObject))

(fn GetMeshComponent
  (return 0))

(fn PaintObject
  (bind _mymeshcomponent (CallFunction|GetMeshComponent))
  (bind _ballcolor (CallFunction|GetColorfromPlayerIndex (Variables|/Game/Blueprints/BP_PlayerState.BP_PlayerState_C|GetPlayerIndex (Variables|Default|GetOwnerPlayerState))))
  (Utilities|IsValid _mymeshcomponent
    (:Is%20Valid
      (Rendering|Material|SetVectorParameterValueonMaterials _mymeshcomponent "Color" (Math|Conversions|ToVector(LinearColor) _ballcolor)))
    (:Is%20Not%20Valid
      (Development|PrintString (Utilities|String|Append "In object : " (Utilities|GetDisplayName self) " while trying to paint have no mesh!")))))

(fn GetPlacableCollision
  (return 0))

(fn CheckIsValidPosition
  (bind _placementblockingcollision (Variables|Default|GetPlacementBlockingCollision))
  (bind _outactors (Collision|SphereOverlapActors (Transformation|GetWorldLocation _placementblockingcollision) (.SphereRadius (Collision|GetComponentBounds _placementblockingcollision)) (Utilities|Array|MakeArray "ObjectTypeQuery7") "PlacableObjectBase_C" (Utilities|Array|MakeArray self)))
  (bind _output_get (Variables|Default|SetIsValidPosition (or (not (Math|Conversions|ToBoolean(Integer) (Utilities|Array|Length _outactors))) (not (Variables|Default|GetPlacedInThisBuildingPhase)))))
  (CallFunction|OnIsValidPositionChanged)
  (return _output_get))

(fn OnRepIsValidPosition
  (CallFunction|OnIsValidPositionChanged))
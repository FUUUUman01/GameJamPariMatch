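; Base placeable object that can move, with an IsMoving state that is reset when the game enters the build phase.
; On the authority, BeginPlay binds StopOnBuild to the game state's phase change.
; StopOnBuild clears IsMoving and passes the current transform to UpdatePosition, which sets X, Z and rotation while keeping Y.
; The file holds no movement logic, and OnRep_StartMoving is empty.
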(event Custom|StopOnBuild
  (params (NewPhase :type EGamePhase%20Enum :default "NewEnumerator2") (OldPhase :type EGamePhase%20Enum :default "NewEnumerator2"))
  (bind _returnvalue (Transformation|GetActorLocation))
  (if (Utilities|Enum|Equal(Enum) NewPhase "NewEnumerator0")
    (Variables|Default|SetbIsMoving false)
    (CallFunction|UpdatePosition (.x _returnvalue) (.z _returnvalue) (Transformation|GetActorRotation))))

(event Custom|UpdatePosition
  (params (X :type Float%20%28single-precision%29) (Z :type Float%20%28single-precision%29) (Rotation :type Rotator))
  (Variables|Default|SetbIsMoving false)
  (Transformation|SetActorLocation (Math|Vector|MakeVector X (.y (Transformation|GetActorLocation)) Z) false false)
  (Transformation|SetActorRotation Rotation))

(event EventBeginPlay
  (|CallParentFunction)
  (Networking|SwitchHasAuthority
    (:Authority
      (bind _asbp_game_state (Utilities|Casting|CastToBP_GameState (Game|GetGameState)))
      (EventDispatchers|BindEventtoOnGamePhaseChanged _asbp_game_state (delegate Custom|StopOnBuild)))))

(event Collision|EventActorBeginOverlap
  (params (OtherActor :type Actor%20Object%20Reference))
  (|CallParentFunction OtherActor) ; This node is disabled and will not be called.\nDrag off pins to build functionality.
)

(event EventTick
  (params (DeltaSeconds :type Float%20%28single-precision%29))
  (|CallParentFunction DeltaSeconds) ; This node is disabled and will not be called.\nDrag off pins to build functionality.
)

(fn ConstructionScript
  (|CallParentFunction))

(fn OnRepStartMoving)

(fn SetIsMoving
  (params (NewIsMoving :type Boolean))
  (Variables|Default|SetbIsMoving NewIsMoving))
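; BP_Bioms is a swipe-style biome selector that slides a row of biomes along Y and exposes the active one.
; NextBiom and PrevBiom step through SetBiomId, which sets the root's target offset from index times spacing and ignores steps past either end.
; Tick eases BiomsRoot toward that target with VInterpTo at SwipeSpeed.
; SetBiomId clamps only for its change check, storing the raw index.
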(event EventTick
  (params (DeltaSeconds :type Float%20%28single-precision%29))
  (if (Math|Vector|NotEqual(Vector) (Variables|/Script/Engine.SceneComponent|GetRelativeLocation (Variables|Default|GetBiomsRoot)) (Variables|Default|GetBiomsRootTargetLocation) 1.0)
    (Transformation|SetRelativeLocation (Variables|Default|GetBiomsRoot) (Math|Interpolation|VInterpTo (Variables|/Script/Engine.SceneComponent|GetRelativeLocation (Variables|Default|GetBiomsRoot)) (Variables|Default|GetBiomsRootTargetLocation) DeltaSeconds (Variables|Default|GetSwipeSpeed)) false false)))

(fn ConstructionScript)

(fn NextBiom
  (CallFunction|SetBiomId (+ (Variables|Default|GetCurrentBiomId) 1)))

(fn PrevBiom
  (CallFunction|SetBiomId (+ (Variables|Default|GetCurrentBiomId) -1)))

(fn SetBiomId
  (params (BiomId :type Integer))
  (if (!= (Math|Integer|Clamp(Integer) BiomId 0 (- (Utilities|Array|Length (Variables|Default|GetBioms)) 1)) (Variables|Default|GetCurrentBiomId))
    (Variables|Default|SetCurrentBiomId BiomId)
    (Variables|Default|SetBiomsRootTargetLocation (Math|Vector|MakeVector 0.0 (* (Variables|Default|GetCurrentBiomId) (LocalVariables|GetDistBetweenBioms)) 0.0))))

(fn GetActiveBiom
  (return (Utilities|Array|Get(acopy) (Variables|Default|GetBioms) (Variables|Default|GetCurrentBiomId))))
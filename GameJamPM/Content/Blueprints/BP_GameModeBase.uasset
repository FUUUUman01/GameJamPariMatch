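; Game mode for a multiplayer ball game that cycles players through waiting, timed building, playing and win phases, relaying changes through BP_GameState.
; On login it funds each player and assigns a ball spawner; once all are ready, it randomly reassigns build grids.
; When everyone finishes building or time expires, it removes invalid placements, spawns balls and starts movable objects.
; The first finished ball wins, triggering a delayed restart into building.
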(event Custom|StartPlayingPhase
  (Utilities|FlowControl|Sequence
    (:then_0
      (bind _outactors (Actor|GetAllActorsOfClass "/Game/Blueprints/PlacableObjects/PlacableObjectBase.PlacableObjectBase_C"))
      (for _array_element _outactors
        (bind _isvalidposition (Default|CheckIsValidPosition _array_element))
        (if (not _isvalidposition)
          (Actor|DestroyActor _array_element))))
    (:then_1
      (CallFunction|ChangeGamePhase "NewEnumerator1")
      (for _array_element_2 (Variables|Default|GetBallSpawners)
        (if (Default|HasValidPlayerStateOwner _array_element_2)
          (Default|Spawn _array_element_2))))
    (:then_2
      (bind _outactors_2 (Actor|GetAllActorsOfClass "/Game/Blueprints/PlacableObjects/MovablePlacableObject.MovablePlacableObject_C"))
      (for _array_element_3 _outactors_2
        (Default|SetIsMoving _array_element_3 true)))))

(event Custom|RestartGame
  (bind _outactors (Actor|GetAllActorsOfClass "/Game/Blueprints/Ball.Ball_C"))
  (for _array_element _outactors
    (Actor|DestroyActor _array_element))
  (CallFunction|StartBuildingPhase)
  (for _array_element_2 (Variables|Default|GetPlayerStates)
    (Variables|/Game/Blueprints/BP_PlayerState.BP_PlayerState_C|SetIsReady _array_element_2 false)))

(event Custom|BallFinished
  (params (BallFinished :type Ball%20Object%20Reference))
  (bind _ownerplayerstate (Variables|/Game/Blueprints/Ball.Ball_C|GetOwnerPlayerState BallFinished))
  (if (Utilities|Enum|Equal(Enum) (Variables|Default|GetCurrentGamePhase) "NewEnumerator1")
    (Development|PrintString "BALL FINISHED")
    (Development|PrintString (Utilities|GetDisplayName _ownerplayerstate))
    (bind _asbp_game_state (Utilities|Casting|CastToBP_GameState (Game|GetGameState)))
    (Default|OnPlayerWinClient _asbp_game_state _ownerplayerstate)
    (CallFunction|ChangeGamePhase "NewEnumerator3")
    (Utilities|FlowControl|Delay (Variables|Default|GetAfterPlayerWinPhaseWait))
    (CallFunction|RestartGame)))

(event Custom|OnPlayerReady
  (params (NewReady :type Boolean))
  (if (Utilities|Enum|Equal(Enum) (Variables|Default|GetCurrentGamePhase) "NewEnumerator2")
    (bind _iseveryoneready (CallFunction|CheckifEveryPlayerIsReady))
    (if _iseveryoneready
      (CallFunction|StartBuildingPhase))))

(event Custom|StartBuildingPhase
  (CallFunction|ChangeGamePhase "NewEnumerator0")
  (CallFunction|ShufflePlayerGrids)
  (CallFunction|WaitforPlayerstoBuildorTimerGoOut))

(event Custom|OnPlayerShouldStopBuilidng
  (params (Player :type BP%20Player%20Controller%20Object%20Reference))
  (EventDispatchers|UnbindEventfromOnClientStoppedBuildingServer Player (delegate Custom|OnPlayerShouldStopBuilidng))
  (if (CallFunction|CheckifEveryPlayerIsStoppedBuilding)
    (Utilities|Time|ClearandInvalidateTimerbyHandle (Variables|Default|GetPlayerBuildingTimerHandle))
    (CallFunction|StartPlayingPhase)))

(event Custom|WaitForPlayersToBuildOrTimerGoOut
  (bind _buildingtime (Variables|Default|GetBuildingTime))
  (for _array_element (Variables|Default|GetPlayerControllers)
    (Default|EnterBuildingModServer _array_element _buildingtime)
    (EventDispatchers|BindEventtoOnClientStoppedBuildingServer _array_element (delegate Custom|OnPlayerShouldStopBuilidng)))
  (bind _returnvalue (Utilities|Time|SetTimerbyEvent (delegate Custom|OnTimeOut) _buildingtime))
  (Variables|Default|SetPlayerBuildingTimerHandle _returnvalue))

(event Custom|OnTimeOut
  (if (Utilities|Enum|NotEqual(Enum) (Variables|Default|GetCurrentGamePhase) "NewEnumerator1")
    (Utilities|Time|ClearandInvalidateTimerbyHandle (Variables|Default|GetPlayerBuildingTimerHandle))
    (for _array_element (Variables|Default|GetPlayerControllers)
      (EventDispatchers|UnbindEventfromOnClientStoppedBuildingServer _array_element (delegate Custom|OnPlayerShouldStopBuilidng))
      (Variables|/Game/Blueprints/BP_PlayerController.BP_PlayerController_C|SetbIsBuilding _array_element false)
      (Default|ExitBuildingMod _array_element))
    (CallFunction|StartPlayingPhase)))

(event EventBeginPlay
  (bind _playerstates (Variables|Default|GetPlayerStates))
  (bind _ballspawners (Variables|Default|GetBallSpawners))
  (bind _output (Utilities|Array|Get(acopy) _ballspawners))
  (bind _output_2 (Utilities|Array|Get(acopy) _playerstates))
  (Utilities|FlowControl|Sequence
    (:then_0
      (bind _outactors (Actor|GetAllActorsOfClass "/Game/Blueprints/BallSpawner.BallSpawner_C"))
      (for _array_element _outactors
        (Utilities|Array|AddUnique (Variables|Default|GetBallSpawners) _array_element))
      (if (and (Utilities|IsValid _output_2) (Utilities|IsValid _output))
        (Variables|/Game/Blueprints/BallSpawner.BallSpawner_C|SetOwnerPlayerState _output _output_2)))
    (:then_1
      (bind _outactors_2 (Actor|GetAllActorsOfClass "/Game/Blueprints/BuildGrid.BuildGrid_C"))
      (for _array_element_2 _outactors_2
        (Utilities|Array|AddUnique (Variables|Default|GetPlayerGrids) _array_element_2)))))

(event EventPostLogin
  (params (NewPlayer :type Player%20Controller%20Object%20Reference))
  (bind _asbp_player_controller (Utilities|Casting|CastToBP_PlayerController NewPlayer))
  (Utilities|Array|Add (Variables|Default|GetPlayerControllers) _asbp_player_controller)
  (bind _asbp_player_state (Utilities|Casting|CastToBP_PlayerState (Variables|/Script/Engine.Controller|GetPlayerState _asbp_player_controller)))
  (Default|SetMoney _asbp_player_state (Variables|Default|GetDefaultPlayerMoney))
  (bind _returnvalue (Utilities|Array|AddUnique (Variables|Default|GetPlayerStates) _asbp_player_state))
  (Variables|/Game/Blueprints/BP_PlayerState.BP_PlayerState_C|SetPlayerIndex _asbp_player_state _returnvalue)
  (EventDispatchers|BindEventtoOnReadyChanged _asbp_player_state (delegate Custom|OnPlayerReady))
  (bind _array_element (Utilities|Array|ForEachLoopwithBreak (Variables|Default|GetBallSpawners) :!label _label)
    (:LoopBody
      (if (not (Default|HasValidPlayerStateOwner _array_element))
        (Variables|/Game/Blueprints/BallSpawner.BallSpawner_C|SetOwnerPlayerState _array_element _asbp_player_state)
        (goto _label Break)))))

(fn ConstructionScript)

(fn CheckifEveryPlayerIsReady
  (for _array_element (Variables|Default|GetPlayerStates)
    (if (not (Variables|/Game/Blueprints/BP_PlayerState.BP_PlayerState_C|GetIsReady _array_element))
      (return false)))
  (return true))

(fn ChangeGamePhase
  (params (NewGamePhase :type EGamePhase%20Enum :default "NewEnumerator2"))
  (bind _asbp_game_state (Utilities|Casting|CastToBP_GameState (Game|GetGameState)))
  (Default|OnGamePhaseChangedClient _asbp_game_state NewGamePhase (Variables|Default|GetCurrentGamePhase))
  (Variables|Default|SetCurrentGamePhase NewGamePhase))

(fn SetMoneyforAllPlayers
  (params (NewMoney :type Integer))
  (for _array_element (Variables|Default|GetPlayerStates)
    (Default|SetMoney _array_element NewMoney)))

(fn CheckifEveryPlayerIsStoppedBuilding
  (for _array_element (Variables|Default|GetPlayerControllers)
    (if (Variables|/Game/Blueprints/BP_PlayerController.BP_PlayerController_C|GetbIsBuilding _array_element)
      (return false)))
  (return true))

(fn ShufflePlayerGrids
  (bind _playergrids (Variables|Default|GetPlayerGrids))
  (LocalVariables|SetCurrentPlayerStates (Variables|Default|GetPlayerStates))
  (Utilities|Array|Shuffle _playergrids)
  (for _array_element _playergrids
    (Variables|/Game/Blueprints/BuildGrid.BuildGrid_C|GetOwnerPlayerState _array_element
      (:then
        _)
      (:else
        _))
    (bind _output_get (Variables|/Game/Blueprints/BuildGrid.BuildGrid_C|SetOwnerPlayerState _array_element (CallFunction|GetRandomPlayerState 0 (LocalVariables|GetCurrentPlayerStates))))
    (Utilities|Array|RemoveItem (LocalVariables|GetCurrentPlayerStates) _output_get)
    (Utilities|IsValid (Variables|/Game/Blueprints/BuildGrid.BuildGrid_C|GetOwnerPlayerState _array_element)
      (:Is%20Valid
        (Development|PrintString "PAINT!")))))

(fn GetRandomPlayerState
  (params (ExcludingPlayerState :type BP%20Player%20State%20Object%20Reference) (PlayerStatesToChooseFrom :type Array%20of%20BP%20Player%20State%20Object%20References))
  (LocalVariables|SetTempPlayerStates PlayerStatesToChooseFrom)
  (return (Utilities|Array|Get(acopy) (LocalVariables|GetTempPlayerStates) (Math|Random|RandomIntegerinRange 0 (- (Utilities|Array|Length (LocalVariables|GetTempPlayerStates)) 1)))))
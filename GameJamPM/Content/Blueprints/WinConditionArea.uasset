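; WinConditionArea is a trigger actor that marks where balls finish.
; When a Ball overlaps its Box on the server, it checks a FinishedBalls array so each ball counts only once.
; A new ball is added to that array and reported to BP_GameModeBase through BallFinished.
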(event OnComponentBeginOverlap(Box)
  (params (OverlappedComponent :type Primitive%20Component%20Object%20Reference) (OtherActor :type Actor%20Object%20Reference) (OtherComp :type Primitive%20Component%20Object%20Reference) (OtherBodyIndex :type Integer) (bFromSweep :type Boolean) (SweepResult :type Hit%20Result%20Structure%20%28by%20ref%29))
  (Networking|SwitchHasAuthority
    (:Authority
      (bind _asball (Utilities|Casting|CastToBall OtherActor))
      (if (== (Utilities|Array|FindItem (Variables|Default|GetFinishedBalls) _asball) -1)
        (bind _asbp_game_mode_base (Utilities|Casting|CastToBP_GameModeBase (Game|GetGameMode)))
        (Utilities|Array|AddUnique (Variables|Default|GetFinishedBalls) _asball)
        (Default|BallFinished _asbp_game_mode_base _asball)))))

(event EventBeginPlay)

(event Collision|EventActorBeginOverlap
  (params (OtherActor :type Actor%20Object%20Reference)))

(event EventTick
  (params (DeltaSeconds :type Float%20%28single-precision%29)))

(fn ConstructionScript)
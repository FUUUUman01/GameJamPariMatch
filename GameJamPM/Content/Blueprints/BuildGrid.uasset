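; BuildGrid is an actor whose Cube mesh is tinted to show which player owns it.
; When the replicated OwnerPlayerState changes, its OnRep calls Paint, which looks up the owner's color by PlayerIndex.
; Paint adds a desaturated copy to the original color and writes the sum to the material's Color vector parameter, using black when no valid owner exists.
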(event Custom|Paint
  (bind _cube (Variables|Default|GetCube))
  (bind _ownerplayerstate (Variables|Default|GetOwnerPlayerState))
  (Utilities|IsValid _ownerplayerstate
    (:Is%20Valid
      (bind _ballcolor (CallFunction|GetColorfromPlayerIndex (Variables|/Game/Blueprints/BP_PlayerState.BP_PlayerState_C|GetPlayerIndex _ownerplayerstate)))
      (Rendering|Material|SetVectorParameterValueonMaterials _cube "Color" (Math|Conversions|ToVector(LinearColor) (+ (Class|KismetMathLibrary|LinearColorDesaturated _ballcolor 0.7) (Class|KismetMathLibrary|LinearColortoNewOpacity _ballcolor 0.2)))))
    (:Is%20Not%20Valid
      (Rendering|Material|SetVectorParameterValueonMaterials _cube "Color" "0, 0, 0"))))

(event Collision|EventActorBeginOverlap
  (params (OtherActor :type Actor%20Object%20Reference)))

(fn ConstructionScript)

(fn OnRepOwnerPlayerState
  (CallFunction|Paint))
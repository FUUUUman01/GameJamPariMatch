(event EventBeginPlay)

(event EventTick
  (params (DeltaSeconds :type Float%20%28single-precision%29)))

(fn ConstructionScript)

(fn ToggleBuildingMode)

(fn SelectPlacableObject
  (params (Object :type Placable%20Object%20Base%20Object%20Reference)))

(fn DeselectPlacableObject)

(fn TrySelectObject
  (params (TrySelectObject :type Placable%20Object%20Base%20Object%20Reference))
  (Variables|/Game/Blueprints/PlacableObjects/PlacableObjectBase.PlacableObjectBase_C|GetOwnerPlayerState TrySelectObject
    (:then
      (if (and (!= TrySelectObject (Variables|Default|GetCurrentSelectedObject)) (== (Variables|/Game/Blueprints/BP_PlayerState.BP_PlayerState_C|GetPlayerIndex (.AsBP%20Player%20State (Utilities|Casting|CastToBP_PlayerState (Variables|GetPlayerState)))) (Variables|/Game/Blueprints/BP_PlayerState.BP_PlayerState_C|GetPlayerIndex (Variables|/Game/Blueprints/PlacableObjects/PlacableObjectBase.PlacableObjectBase_C|GetOwnerPlayerState TrySelectObject))))
        (CallFunction|SelectPlacableObject TrySelectObject)
        (else
          (CallFunction|DeselectPlacableObject))))
    (:else)))

(fn IsMineBuildingGrid
  (params (Grid :type Actor%20Object%20Reference))
  (bind _asbuild_grid (Utilities|Casting|CastToBuildGrid Grid)
    (:then
      (return (== (Variables|/Game/Blueprints/BuildGrid.BuildGrid_C|GetOwnerPlayerState _asbuild_grid) (Variables|GetPlayerState))))
    (:CastFailed
      (return false))))